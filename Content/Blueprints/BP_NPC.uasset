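; BP_NPC is a character that patrols back and forth along an array of waypoints.
; BeginPlay snaps it to the first waypoint and sets walk speed from MovementSpeed.
; While that speed is positive, Tick adds movement input toward the next waypoint and, within WaypointStopDistance, advances the index, reversing direction at either end of the array.
; An alternative lerp-based mover, LerpToNextWaypoint, is defined but never called.
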(event EventTick
  (params (DeltaSeconds :type Float%20%28single-precision%29))
  (if (> (Variables|Default|GetMovementSpeed) 0.0)
    (CallFunction|MovetoNextWaypoint)
    (bind _returnvalue (CallFunction|IsNextWaypointReached))
    (if _returnvalue
      (CallFunction|UpdateNextWaypoint))))

(event EventBeginPlay
  (bind _waypoints (Variables|Default|GetWaypoints))
  (if (Utilities|Array|IsNotEmpty _waypoints)
    (Transformation|SetActorLocation (Utilities|Array|Get(acopy) _waypoints) false false)
    (Variables|/Script/Engine.CharacterMovementComponent|SetMaxWalkSpeed (Variables|Character|GetCharacterMovement) (Variables|Default|GetMovementSpeed))))

(fn ConstructionScript)

(fn LerptoNextWaypoint
  (bind _waypoints (Variables|Default|GetWaypoints))
  (bind _nextwaypointindex (Variables|Default|GetNextWaypointIndex))
  (bind _waypoints_2 (Variables|Default|GetWaypoints))
  (bind _output (Utilities|Array|Get(acopy) _waypoints _nextwaypointindex))
  (LocalVariables|SetTotalDistance (Math|Vector|Distance(Vector) (Utilities|Array|Get(acopy) _waypoints (Variables|Default|GetPrevWaypointIndex)) _output))
  (bind _output_get (LocalVariables|SetRemainingDistance (Math|Vector|Distance(Vector) _output (Transformation|GetActorLocation))))
  (Transformation|SetActorLocation (Math|Vector|Lerp(Vector) (Utilities|Array|Get(acopy) _waypoints_2 (Variables|Default|GetPrevWaypointIndex)) (Utilities|Array|Get(acopy) _waypoints_2 (Variables|Default|GetNextWaypointIndex)) (- 1.0 (Math|Interpolation|FInterptoConstant (/ _output_get (LocalVariables|GetTotalDistance)) 0.0 (Utilities|Time|GetWorldDeltaSeconds) (Variables|Default|GetMovementSpeed)))) false false))

(fn IsNextWaypointReached
  (return (<= (Math|Vector|Distance(Vector) (Transformation|GetActorLocation) (Utilities|Array|Get(acopy) (Variables|Default|GetWaypoints) (Variables|Default|GetNextWaypointIndex))) (Variables|Default|GetWaypointStopDistance))))

(fn UpdateNextWaypoint
  (LocalVariables|SettraversalDirection (- (Variables|Default|GetNextWaypointIndex) (Variables|Default|GetPrevWaypointIndex)))
  (if (or (== (Variables|Default|GetNextWaypointIndex) (- (Utilities|Array|Length (Variables|Default|GetWaypoints)) 1)) (== (Variables|Default|GetNextWaypointIndex) 0))
    (LocalVariables|SettraversalDirection (* (LocalVariables|GettraversalDirection) -1)))
  (Variables|Default|SetPrevWaypointIndex (Variables|Default|GetNextWaypointIndex))
  (Variables|Default|SetNextWaypointIndex (+ (Variables|Default|GetNextWaypointIndex) (LocalVariables|GettraversalDirection))))

(fn MovetoNextWaypoint
  (Pawn|Input|AddMovementInput (Math|Vector|GetUnitDirection(Vector) (Transformation|GetActorLocation) (Utilities|Array|Get(acopy) (Variables|Default|GetWaypoints) (Variables|Default|GetNextWaypointIndex))) 1.0 false))