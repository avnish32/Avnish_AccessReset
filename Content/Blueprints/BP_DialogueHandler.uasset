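; BP_DialogueHandler is an actor that passes dialogue messages to the player's BP_HUD and closes the dialogue panel when dialogue ends.
; On BeginPlay it resets its next-dialogue dispatcher and caches the first player's HUD.
; SendDialogueToHUD shows the panel with itself as handler.
; By default the dispatcher is bound to OnLastDialogue, which hides the panel; the reset event clears other bindings to restore that default.
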(event Custom|OnLastDialogue
  (CallFunction|EndDialogue))

(event Custom|ResetOnNextDialogueBehaviour
  (EventDispatchers|UnbindallEventsfromOnNextDialogueDispatcher)
  (EventDispatchers|BindEventtoOnNextDialogueDispatcher (delegate Custom|OnLastDialogue)))

(event EventBeginPlay
  (Utilities|FlowControl|Sequence
    (:then_0
      (CallFunction|ResetonNextDialogueBehaviour))
    (:then_1
      (bind _asbp_hud (Utilities|Casting|CastToBP_HUD (HUD|GetHUD (Game|GetPlayerController 0))))
      (Variables|Default|SetHUD _asbp_hud))))

(event Collision|EventActorBeginOverlap
  (params (OtherActor :type Actor%20Object%20Reference)))

(event EventTick
  (params (DeltaSeconds :type Float%20%28single-precision%29)))

(fn ConstructionScript)

(fn SendDialoguetoHUD
  (params (DialogueMsg :type String))
  (Default|ShowDialoguePanel (Variables|Default|GetHUD) DialogueMsg self))

(fn EndDialogue
  (Default|HideDialoguePanel (Variables|Default|GetHUD)))