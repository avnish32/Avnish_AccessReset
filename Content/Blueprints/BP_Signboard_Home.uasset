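; Home building signboard, a child of a signboard base class, that lets the player enter home to rest.
; BeginPlay sets up the building timings and a game-parameter map, then binds the building-entered event.
; On entry, rest time and energy gain from the event's params overwrite that map before the open check and entry.
; The CreateBuildingPanel override has the HUD show the home panel unless the parent call returns true.
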(event Custom|OnHomeEntered
  (params (ParamsMap :type Map%20of%20Strings%20to%20Reals))
  (CallFunction|UpdateParamsandValuesBasedonRestPeriod ParamsMap)
  (CallFunction|CheckifOpenandEnter))

(event EventBeginPlay
  (bind _buildinginfo (Variables|Default|GetBuildingInfo))
  (bind _timings (Utilities|Struct|BreakS_BuildingInfo _buildinginfo))
  (|CallParentFunction)
  (Utilities|FlowControl|Sequence
    (:then_0
      (Utilities|Array|Add :TargetArray _timings)
      (Utilities|Array|Add :TargetArray _timings))
    (:then_1
      (Variables|Default|SetParamsAndValues (Utilities|Map|MakeMap (Utilities|Enum|LiteralenumE_GameParams "NewEnumerator1") (Math|Float|MakeLiteralFloat 0.0) "NewEnumerator2" 0.0)))
    (:then_2
      (EventDispatchers|UnbindallEventsfromOnBuildingEntered)
      (EventDispatchers|BindEventtoOnBuildingEntered (delegate Custom|OnHomeEntered)))))

(event Collision|EventActorBeginOverlap
  (params (OtherActor :type Actor%20Object%20Reference)))

(event EventTick
  (params (DeltaSeconds :type Float%20%28single-precision%29)))

(fn ConstructionScript
  (|CallParentFunction))

(fn CreateBuildingPanel
  (bind _ispanelcreated (|CallParentFunction))
  (if _ispanelcreated
    (return false)
    (else
      (Default|ShowHomeBuildingPanel (Variables|Default|GetHUD) (Variables|Default|GetParamsAndValues) self))))

(fn UpdateParamsandValuesBasedonRestPeriod
  (params (RestPeriodParamsMap :type Map%20of%20Strings%20to%20Reals))
  (bind _paramsandvalues (Variables|Default|GetParamsAndValues))
  (Utilities|Map|Add _paramsandvalues "NewEnumerator1" (.Value (Utilities|Map|Find RestPeriodParamsMap "RestPeriodTimeInMins")))
  (Utilities|Map|Add _paramsandvalues "NewEnumerator2" (.Value (Utilities|Map|Find RestPeriodParamsMap "EnergyFromRest"))))