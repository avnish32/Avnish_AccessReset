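; Pharmacy signboard Blueprint, a child of a shared signboard parent, that handles entering the pharmacy building.
; On the building-entered event it runs the open check and enter, and its panel override shows the HUD building panel when the parent call returns false.
; Difficulty scaling rebuilds values from the Normal baseline, multiplying Money and Time by the parent's factor and dividing Energy by it, rounded to two decimals.
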(event Custom|OnPharmacyEntered
  (params (ParamsMap :type Map%20of%20Strings%20to%20Reals))
  (CallFunction|CheckifOpenandEnter))

(event EventBeginPlay
  (|CallParentFunction)
  (EventDispatchers|BindEventtoOnBuildingEntered (delegate Custom|OnPharmacyEntered)))

(fn ConstructionScript
  (|CallParentFunction))

(fn CreateBuildingPanel
  (bind _ispanelcreated (|CallParentFunction))
  (if (not _ispanelcreated)
    (Default|ShowOpenBuildingPanel (Variables|Default|GetHUD) self (Variables|Default|GetParamsAndValues))
    (return false)))

(fn GetPostExitDialogues
  (|CallParentFunction)
  (return (Variables|Default|GetPostExitDialogues)))

(fn UpdateParamsandValuesbyDifficulty
  (bind _paramsandvalues (Variables|Default|GetParamsAndValues))
  (bind _penalty_modifier_out (|CallParentFunction))
  (bind _keys (Utilities|Map|Keys (Variables|Default|GetParamsAndValues)))
  (for _array_element _keys
    (switch Utilities|FlowControl|Switch|SwitchonE_GameParams _array_element
      (:NewEnumerator0
        (bind _floatout (CallFunction|Roundto2DecimalPlaces (* (.Value (Utilities|Map|Find (Variables|Default|GetParamsAndValuesForNormal) _array_element)) _penalty_modifier_out) :!label _label))
        (Utilities|Map|Add _paramsandvalues _array_element _floatout))
      (:NewEnumerator1
        (goto _label))
      (:NewEnumerator2
        (bind _floatout_2 (CallFunction|Roundto2DecimalPlaces (/ (.Value (Utilities|Map|Find (Variables|Default|GetParamsAndValuesForNormal) _array_element)) _penalty_modifier_out)))
        (Utilities|Map|Add _paramsandvalues _array_element _floatout_2))))
  (return _penalty_modifier_out))