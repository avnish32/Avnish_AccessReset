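; Signboard for the player's home building, where resting changes game time and stats such as energy.
; It opens the home HUD panel, and its entered event takes the chosen rest period and energy gain before the open-and-enter check.
; Difficulty scales rest via a stat-based clamped remap: Easy can wake the player early, Hard can cause oversleeping, each adjusting another parameter.
; Post-exit dialogue prepends the matching message.
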(event Custom|OnHomeEntered
  (params (ParamsMap :type Map%20of%20Strings%20to%20Reals))
  (CallFunction|UpdateParamsandValuesBasedonRestPeriodandDifficulty ParamsMap)
  (CallFunction|CheckifOpenandEnter))

(event EventBeginPlay
  (bind _buildinginfo (Variables|Default|GetBuildingInfo))
  (bind _timings (Utilities|Struct|BreakS_BuildingInfo _buildinginfo))
  (|CallParentFunction)
  (Utilities|FlowControl|Sequence
    (:then_0
      (Utilities|Array|Add :TargetArray _timings)
      (Utilities|Array|Add :TargetArray _timings))
    (:then_1
      (Variables|Default|SetParamsAndValues (Utilities|Map|MakeMap (Utilities|Enum|LiteralenumE_GameParams "NewEnumerator1") (Math|Float|MakeLiteralFloat 0.0) "NewEnumerator2" 0.0)))
    (:then_2
      (EventDispatchers|UnbindallEventsfromOnBuildingEntered)
      (EventDispatchers|BindEventtoOnBuildingEntered (delegate Custom|OnHomeEntered)))))

(event Collision|EventActorBeginOverlap
  (params (OtherActor :type Actor%20Object%20Reference)))

(event EventTick
  (params (DeltaSeconds :type Float%20%28single-precision%29)))

(fn ConstructionScript
  (|CallParentFunction))

(fn CreateBuildingPanel
  (bind _ispanelcreated (|CallParentFunction))
  (if _ispanelcreated
    (return false)
    (else
      (CallFunction|ResetDifficultyBasedChanges)
      (Default|ShowHomeBuildingPanel (Variables|Default|GetHUD) (Variables|Default|GetParamsAndValues) self))))

(fn UpdateParamsandValuesBasedonRestPeriodandDifficulty
  (params (RestPeriodParamsMap :type Map%20of%20Strings%20to%20Reals))
  (bind _value (Utilities|Map|Find RestPeriodParamsMap "RestPeriodTimeInMins"))
  (bind _gamestats (Variables|Default|GetGameStats))
  (bind _paramsandvalues (Variables|Default|GetParamsAndValues))
  (bind _currentdifficulty (Variables|/Game/Blueprints/BP_GameStats.BP_GameStats_C|GetCurrentDifficulty _gamestats))
  (bind _stats (Variables|/Game/Blueprints/BP_GameStats.BP_GameStats_C|GetStats _gamestats))
  (bind (_difficultyenum _desc _penaltymodifier) (Utilities|Struct|BreakS_DifficultyMode _currentdifficulty))
  (bind _value_2 (Utilities|Map|Find _stats "NewEnumerator2"))
  (bind _returnvalue (- 5e+01 _value_2))
  (bind _returnvalue_2 (- _value_2 5e+01))
  (bind _returnvalue_3 (Math|Float|MapRangeClamped _returnvalue_2 0.0 5e+01 1.0 _penaltymodifier))
  (bind _returnvalue_4 (Math|Float|MapRangeClamped _returnvalue 0.0 5e+01 1.0 _penaltymodifier))
  (switch Utilities|FlowControl|Switch|SwitchonE_DiffcultyModes _difficultyenum
    (:NewEnumerator0
      (Variables|Default|SetWokeUpEarly (< _returnvalue_3 1.0))
      (Utilities|Map|Add _paramsandvalues "NewEnumerator1" (* _returnvalue_3 _value))
      (Utilities|Map|Add (Variables|Default|GetParamsAndValues) "NewEnumerator4" (/ 2.0 _returnvalue_3)))
    (:NewEnumerator1
      (Utilities|Map|Add _paramsandvalues "NewEnumerator1" _value))
    (:NewEnumerator2
      (Variables|Default|SetOverslept (> _returnvalue_4 1.0))
      (Utilities|Map|Add _paramsandvalues "NewEnumerator1" (* _returnvalue_4 _value))
      (Utilities|Map|Add (Variables|Default|GetParamsAndValues) "NewEnumerator4" (* _returnvalue_4 -5.0))))
  (Utilities|Map|Add _paramsandvalues "NewEnumerator2" (.Value (Utilities|Map|Find RestPeriodParamsMap "EnergyFromRest"))))

(fn GetPostExitDialogues
  (bind _postexitdialogues (Variables|Default|GetPostExitDialogues))
  (bind _resultantdialogues (LocalVariables|GetResultantDialogues))
  (|CallParentFunction)
  (Utilities|Array|Clear (LocalVariables|GetResultantDialogues))
  (if (Variables|Default|GetOverslept)
    (Utilities|Array|Add (LocalVariables|GetResultantDialogues) (Variables|Default|GetOversleptMsg))
    (for _array_element _postexitdialogues
      (Utilities|Array|Add (LocalVariables|GetResultantDialogues) _array_element))
    (return _resultantdialogues)
    (elif (Variables|Default|GetWokeUpEarly)
      (Utilities|Array|Add (LocalVariables|GetResultantDialogues) (Variables|Default|GetWokeUpEarlyMsg))
      (for _array_element_2 _postexitdialogues
        (Utilities|Array|Add _resultantdialogues _array_element_2))
      (return (LocalVariables|GetResultantDialogues))
      (else
        (return (Variables|Default|GetPostExitDialogues))))))

(fn ResetDifficultyBasedChanges
  (Variables|Default|SetOverslept false)
  (Variables|Default|SetWokeUpEarly false)
  (Utilities|Map|Remove (Variables|Default|GetParamsAndValues) "NewEnumerator4"))