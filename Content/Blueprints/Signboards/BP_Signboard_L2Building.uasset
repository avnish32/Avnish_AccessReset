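; Signboard for a Level 2 building that shows a restaurant panel through the HUD.
; On entry it alerts if closed, otherwise snapshots stats and starts the HUD transition; exiting ends it and initiates post-exit dialogues.
; GetPostExitDialogues picks satisfied or unsatisfied lines by whether Energy rose, though its local playback chain is unwired.
; Difficulty updates scale menu Money and Time by the parent's penalty modifier and divide Energy and PYUMO by it.
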(event Custom|OnL2BuildingEntered
  (params (ParamsMap :type Map%20of%20Strings%20to%20Reals))
  (bind _returnvalue (CallFunction|IsBuildingOpen))
  (if _returnvalue
    (Variables|Default|SetStatsBeforeEntering (Variables|/Game/Blueprints/BP_GameStats.BP_GameStats_C|GetStats (Variables|Default|GetGameStats)))
    (Variables|/Game/TopDown/Blueprints/BP_TopDownController.BP_TopDownController_C|SetIsInTransition (Variables|Default|GetTop%20Down%20Controller) true)
    (Default|OnL2BuildingEntered (Variables|Default|GetHUD) self)
    (else
      (Default|RaiseAlert (Variables|Default|GetHUD) (Variables|Default|GetBuildingClosedAlertMsg) 2.0))))

(event Custom|OnL2BuildingExited
  (Variables|/Game/TopDown/Blueprints/BP_TopDownController.BP_TopDownController_C|SetIsInTransition (Variables|Default|GetTop%20Down%20Controller) false)
  (Default|OnL2BuildingExited (Variables|Default|GetHUD))
  (CallFunction|InitiatePostExitDialogues))

(event Custom|AdvanceDialogue
  (bind _result (Math|Integer|IncrementInt (Variables|Default|GetcurrentDialogueIndex))
    (:%20%20
      (Default|SendDialoguetoHUD (Variables|Default|GetDialogueHandler) (Utilities|Array|Get(acopy) (Variables|Default|GetCurrentDialogues) _result))
      (if (== (Variables|Default|GetcurrentDialogueIndex) (- (Utilities|Array|Length (Variables|Default|GetCurrentDialogues)) 1))
        (Default|ResetonNextDialogueBehaviour (Variables|Default|GetDialogueHandler))))))

(event EventBeginPlay
  (|CallParentFunction)
  (EventDispatchers|BindEventtoOnBuildingEntered (delegate Custom|OnL2BuildingEntered)))

(event Collision|EventActorBeginOverlap
  (params (OtherActor :type Actor%20Object%20Reference)))

(event EventTick
  (params (DeltaSeconds :type Float%20%28single-precision%29)))

(fn ConstructionScript
  (|CallParentFunction))

(fn CreateBuildingPanel
  (bind _ispanelcreated (|CallParentFunction))
  (if (not _ispanelcreated)
    (Default|ShowRestaurantPanel (Variables|Default|GetHUD) self)))

(fn HideBuildingPanel
  (Default|HideCurrentBuildingPanel (Variables|Default|GetHUD)))

(fn GetPostExitDialogues
  (if (< (.Value (Utilities|Map|Find (Variables|Default|GetStatsBeforeEntering) "NewEnumerator2")) (.Value (Utilities|Map|Find (Variables|/Game/Blueprints/BP_GameStats.BP_GameStats_C|GetStats (Variables|Default|GetGameStats)) "NewEnumerator2")))
    (return (Variables|Default|GetPlayerSatisfied_Dialogues))
    (else
      (return (Variables|Default|GetPlayerNotSatisfied_Dialogues)))))

(fn UpdateParamsandValuesbyDifficulty
  (bind _penalty_modifier_out (|CallParentFunction))
  (for (_array_element _array_index) (Variables|Default|GetMenu)
    (bind _updatedparamsandvalues (CallFunction|UpdateL2ItemParamsandValuesbyDifficulty (.ParamsAndValues (Utilities|Struct|BreakS_L2Item _array_element)) _penalty_modifier_out))
    (Utilities|Array|SetArrayElem (Variables|Default|GetMenu) _array_index (Utilities|Struct|MakeS_L2Item (.Name (Utilities|Struct|BreakS_L2Item _array_element)) (.Icon (Utilities|Struct|BreakS_L2Item _array_element)) _updatedparamsandvalues (.ConsumptionMode (Utilities|Struct|BreakS_L2Item _array_element)))))
  (Development|PrintString "L2 params updated by diff")
  (return 0.0))

(fn UpdateL2ItemParamsandValuesbyDifficulty
  (params (ParamsAndValuesIn :type Map%20of%20E_GameParams%20Enums%20to%20Reals :default "NewEnumerator0") (PenaltyModifier :type Float%20%28double-precision%29))
  (bind _keys (Utilities|Map|Keys ParamsAndValuesIn))
  (for _array_element _keys
    (switch Utilities|FlowControl|Switch|SwitchonE_GameParams _array_element
      (:NewEnumerator0
        (Utilities|Map|Add ParamsAndValuesIn _array_element (/ (Math|Conversions|ToFloat(Integer) (Math|Float|Floor (* (* (.Value (Utilities|Map|Find ParamsAndValuesIn _array_element)) PenaltyModifier) 1e+02))) 1e+02)))
      (:NewEnumerator1
        (Utilities|Map|Add ParamsAndValuesIn _array_element (Math|Conversions|ToFloat(Integer) (Math|Float|Round (* (.Value (Utilities|Map|Find ParamsAndValuesIn _array_element)) PenaltyModifier)))))
      (:NewEnumerator2
        (Utilities|Map|Add ParamsAndValuesIn _array_element (/ (Math|Conversions|ToFloat(Integer) (Math|Float|Floor (* (/ (.Value (Utilities|Map|Find ParamsAndValuesIn _array_element)) PenaltyModifier) 1e+02))) 1e+02) :!label _label))
      (:NewEnumerator4
        (goto _label))))
  (return ParamsAndValuesIn))