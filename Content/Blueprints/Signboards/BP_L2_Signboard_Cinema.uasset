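; BP_L2_Signboard_Cinema is the cinema signboard Blueprint, supplying the dialogue shown after the player exits.
; GetPostExitDialogues compares one tracked stat's value from before entering with its current GameStats value.
; A drop in that stat returns the satisfied dialogues; otherwise it returns the not-satisfied set.
; The event graph is unused, and the construction script only calls its parent.
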(event EventBeginPlay
  (|CallParentFunction) ; This node is disabled and will not be called.\nDrag off pins to build functionality.
)

(event Collision|EventActorBeginOverlap
  (params (OtherActor :type Actor%20Object%20Reference))
  (|CallParentFunction OtherActor) ; This node is disabled and will not be called.\nDrag off pins to build functionality.
)

(event EventTick
  (params (DeltaSeconds :type Float%20%28single-precision%29))
  (|CallParentFunction DeltaSeconds) ; This node is disabled and will not be called.\nDrag off pins to build functionality.
)

(fn ConstructionScript
  (|CallParentFunction))

(fn GetPostExitDialogues
  (if (> (.Value (Utilities|Map|Find (Variables|Default|GetStatsBeforeEntering) "NewEnumerator0")) (.Value (Utilities|Map|Find (Variables|/Game/Blueprints/BP_GameStats.BP_GameStats_C|GetStats (Variables|Default|GetGameStats)) "NewEnumerator0")))
    (return (Variables|Default|GetPlayerSatisfied_Dialogues))
    (else
      (return (Variables|Default|GetPlayerNotSatisfied_Dialogues)))))