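; BP_Signboard_Learning is a child signboard Blueprint for the Learning building that manages that building's HUD panel.
; On BeginPlay it binds OnBuildingEntered to a handler, named OnWellbeingEntered despite the Learning asset, which calls CheckIfOpenAndEnter.
; Its CreateBuildingPanel override calls the parent first and, if that returns false, shows the HUD's open-building panel with itself and its parameters.
; HideBuildingPanel tells the HUD to hide the current panel.
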(event Custom|OnWellbeingEntered
  (params (ParamsMap :type Map%20of%20Strings%20to%20Reals))
  (CallFunction|CheckifOpenandEnter))

(event EventBeginPlay
  (|CallParentFunction)
  (EventDispatchers|BindEventtoOnBuildingEntered (delegate Custom|OnWellbeingEntered)))

(event EventTick
  (params (DeltaSeconds :type Float%20%28single-precision%29)))

(fn ConstructionScript
  (|CallParentFunction))

(fn CreateBuildingPanel
  (bind _ispanelcreated (|CallParentFunction))
  (if (not _ispanelcreated)
    (Default|ShowOpenBuildingPanel (Variables|Default|GetHUD) self (Variables|Default|GetParamsAndValues))))

(fn HideBuildingPanel
  (Default|HideCurrentBuildingPanel (Variables|Default|GetHUD)))