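; Building signboard actor that gates entry by opening hours, including overnight ranges, and applies the building's stat changes to the player.
; Sphere overlap shows the closed-building panel outside those hours and hides the current panel on exit.
; Entry validates changes with BP_GameStats, runs a timed HUD transition, updates stats, then steps through post-exit dialogue via BP_DialogueHandler.
; GetPostExitDialogues is an empty stub here; BeginPlay also registers the signboard with the minimap.
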(event OnComponentBeginOverlap(SphereCollider)
  (params (OverlappedComponent :type Primitive%20Component%20Object%20Reference) (OtherActor :type Actor%20Object%20Reference) (OtherComp :type Primitive%20Component%20Object%20Reference) (OtherBodyIndex :type Integer) (bFromSweep :type Boolean) (SweepResult :type Hit%20Result%20Structure%20%28by%20ref%29))
  (Utilities|Casting|CastToBP_TopDownCharacter OtherActor)
  (CallFunction|CreateBuildingPanel))

(event OnComponentEndOverlap(SphereCollider)
  (params (OverlappedComponent :type Primitive%20Component%20Object%20Reference) (OtherActor :type Actor%20Object%20Reference) (OtherComp :type Primitive%20Component%20Object%20Reference) (OtherBodyIndex :type Integer))
  (Utilities|Casting|CastToBP_TopDownCharacter OtherActor)
  (Default|HideCurrentBuildingPanel (Variables|Default|GetHUD)))

(event Custom|InitiatePostExitDialogues
  (bind _dialoguehandler (Variables|Default|GetDialogueHandler))
  (Default|HideDialoguePanel (Variables|Default|GetHUD))
  (bind _postexitdialogues (CallFunction|GetPostExitDialogues))
  (if (Utilities|Array|IsNotEmpty _postexitdialogues)
    (Variables|Default|SetCurrentDialogues _postexitdialogues)
    (Variables|Default|SetcurrentDialogueIndex -1)
    (EventDispatchers|UnbindallEventsfromOnNextDialogueDispatcher _dialoguehandler)
    (EventDispatchers|BindEventtoOnNextDialogueDispatcher _dialoguehandler (delegate Custom|AdvanceDialogue))
    (CallFunction|AdvanceDialogue)))

(event Custom|TransitionAndUpdateParams
  (Variables|Default|SetStatsBeforeEntering (Variables|/Game/Blueprints/BP_GameStats.BP_GameStats_C|GetStats (Variables|Default|GetGameStats)))
  (bind (_isvalid _validationmsg) (Default|ValidateStatsBeforeUpdating (Variables|Default|GetGameStats) (Variables|Default|GetParamsAndValues)))
  (if _isvalid
    (Default|OnGenericBuildingEntered (Variables|Default|GetHUD) (Variables|Default|GetTransitionMsg) false)
    (Utilities|FlowControl|Delay 1.0)
    (Variables|/Game/TopDown/Blueprints/BP_TopDownController.BP_TopDownController_C|SetIsInTransition (Variables|Default|GetTop%20Down%20Controller) true)
    (Utilities|FlowControl|Delay 1.0)
    (CallFunction|UpdateGameStats)
    (Development|PrintString "Stats updated")
    (Utilities|FlowControl|Delay 2.0)
    (if (<= (.Value (Utilities|Map|Find (Variables|/Game/Blueprints/BP_GameStats.BP_GameStats_C|GetStats (Variables|Default|GetGameStats)) "NewEnumerator2")) 0.0)
      (Variables|/Game/TopDown/Blueprints/BP_TopDownController.BP_TopDownController_C|SetIsInTransition (Variables|Default|GetTop%20Down%20Controller) false)
      (else
        (Default|OnTransitionCompleted (Variables|Default|GetHUD))
        (CallFunction|InitiatePostExitDialogues)))
    (else
      (Development|PrintString _validationmsg))))

(event Custom|AdvanceDialogue
  (bind _result (Math|Integer|IncrementInt (Variables|Default|GetcurrentDialogueIndex))
    (:%20%20
      (Default|SendDialoguetoHUD (Variables|Default|GetDialogueHandler) (Utilities|Array|Get(acopy) (Variables|Default|GetCurrentDialogues) _result))
      (if (== (Variables|Default|GetcurrentDialogueIndex) (- (Utilities|Array|Length (Variables|Default|GetCurrentDialogues)) 1))
        (Default|ResetonNextDialogueBehaviour (Variables|Default|GetDialogueHandler))))))

(event EventBeginPlay
  (Utilities|FlowControl|Sequence
    (:then_0
      (bind _asbp_hud (Utilities|Casting|CastToBP_HUD (HUD|GetHUD (Game|GetPlayerController 0))))
      (Variables|Default|SetHUD _asbp_hud))
    (:then_1
      (bind _returnvalue (Actor|GetActorOfClass "/Game/Blueprints/BP_GameStats.BP_GameStats_C"))
      (Variables|Default|SetGameStats _returnvalue))
    (:then_2
      (bind _asbp_top_down_controller (Utilities|Casting|CastToBP_TopDownController (Game|GetPlayerController 0)))
      (Variables|Default|SetTop%20Down%20Controller _asbp_top_down_controller))
    (:then_3
      (bind _returnvalue_2 (Actor|GetActorOfClass "/Game/Blueprints/BP_DialogueHandler.BP_DialogueHandler_C"))
      (Variables|Default|SetDialogueHandler _returnvalue_2))
    (:then_4
      (EventDispatchers|UnbindallEventsfromOnBuildingEntered))
    (:then_5
      (Variables|Default|SetParamsAndValuesForNormal (Variables|Default|GetParamsAndValues))
      (Utilities|FlowControl|Delay 0.2)
      (CallFunction|UpdateParamsandValuesbyDifficulty))
    (:then_6
      (Rendering|Components|Sprite|SetSprite (Variables|Default|GetIconBillboard) (Variables|Default|GetSignboardIcon)))
    (:then_7
      (bind _returnvalue_3 (Actor|GetActorOfClass "/Game/Blueprints/BP_MinimapController.BP_MinimapController_C"))
      (Utilities|IsValid _returnvalue_3 :!label _label
        (:Is%20Valid
          (Default|OnSignboardBeginPlay _returnvalue_3 self))
        (:Is%20Not%20Valid
          (Utilities|FlowControl|DelayUntilNextTick)
          (goto _label))))))

(fn ConstructionScript)

(fn UpdateGameStats
  (Default|UpdateStats (Variables|Default|GetGameStats) (Variables|Default|GetParamsAndValues)))

(fn CreateBuildingPanel
  (bind _returnvalue (CallFunction|IsBuildingOpen))
  (if _returnvalue
    (return false)
    (else
      (Default|ShowClosedBuildingPanel (Variables|Default|GetHUD) self)
      (return true))))

(fn HideBuildingPanel
  (Default|HideCurrentBuildingPanel (Variables|Default|GetHUD)))

(fn IsBuildingOpen
  (bind _buildinginfo (Variables|Default|GetBuildingInfo))
  (bind _timings (Utilities|Struct|BreakS_BuildingInfo _buildinginfo))
  (bind _output (Utilities|Array|Get(acopy) _timings 1))
  (bind _output_2 (Utilities|Array|Get(acopy) _timings))
  (bind (_x _y) (Math|Vector2D|BreakVector2D _output))
  (bind (_x_2 _y_2) (Math|Vector2D|BreakVector2D _output_2))
  (if (and (Class|KismetMathLibrary|EqualExactlyVector2DVector2D _output_2) (Class|KismetMathLibrary|EqualExactlyVector2DVector2D _output))
    (return true)
    (else
      (bind _output_get (LocalVariables|SetOpeningTimeInMins (+ (* _x_2 6e+01) _y_2)))
      (bind _output_get_2 (LocalVariables|SetClosingTimeInMins (+ (* _x 6e+01) _y)))
      (LocalVariables|SetCurrentTimeInMins (.Value (Utilities|Map|Find (Variables|/Game/Blueprints/BP_GameStats.BP_GameStats_C|GetStats (Variables|Default|GetGameStats)) "NewEnumerator1")))
      (if (< _output_get _output_get_2)
        (return (and (>= (LocalVariables|GetCurrentTimeInMins) (LocalVariables|GetOpeningTimeInMins)) (<= (LocalVariables|GetCurrentTimeInMins) (LocalVariables|GetClosingTimeInMins))))
        (else
          (return (or (and (<= (LocalVariables|GetCurrentTimeInMins) 1.44e+03) (>= (LocalVariables|GetCurrentTimeInMins) (LocalVariables|GetOpeningTimeInMins))) (and (>= (LocalVariables|GetCurrentTimeInMins) 0.0) (<= (LocalVariables|GetCurrentTimeInMins) (LocalVariables|GetClosingTimeInMins))))))))))

(fn GetPostExitDialogues
  (return 0))

(fn CheckifOpenandEnter
  (bind _returnvalue (CallFunction|IsBuildingOpen))
  (if _returnvalue
    (CallFunction|TransitionandUpdateParams)
    (else
      (Default|RaiseAlert (Variables|Default|GetHUD) (Variables|Default|GetBuildingClosedAlertMsg) 2.0))))

(fn UpdateParamsandValuesbyDifficulty
  (bind _gamestats (Variables|Default|GetGameStats)
    (:then
      (bind _output_get (LocalVariables|SetPenaltyModifier (.PenaltyModifier (Utilities|Struct|BreakS_DifficultyMode (Variables|/Game/Blueprints/BP_GameStats.BP_GameStats_C|GetCurrentDifficulty _gamestats)))))
      (return _output_get))
    (:else
      (Development|PrintString "Game stats invalid on signboard" true true "(R=1.000000,G=0.063568,B=0.000000,A=1.000000)")
      (return 1.0))))

(fn Roundto2DecimalPlaces
  (params (FloatIn :type Float%20%28double-precision%29))
  (return (/ (Math|Conversions|ToFloat(Integer) (Math|Float|Floor (* FloatIn 1e+02))) 1e+02)))