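; Hospital signboard Blueprint, a child of a signboard base class, that lets the player enter and use a hospital building.
; On BeginPlay it binds the building-entered event to an open-check-and-enter call.
; Overrides show the open-building panel on the HUD when the parent's panel creation returns false and supply hospital post-exit dialogue.
; Another override scales Money and Time parameters by the parent's difficulty multiplier, rounded to two decimals.
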(event Custom|OnHospitalEntered
  (params (ParamsMap :type Map%20of%20Strings%20to%20Reals))
  (CallFunction|CheckifOpenandEnter))

(event EventBeginPlay
  (|CallParentFunction)
  (EventDispatchers|BindEventtoOnBuildingEntered (delegate Custom|OnHospitalEntered)))

(fn ConstructionScript
  (|CallParentFunction))

(fn CreateBuildingPanel
  (bind _ispanelcreated (|CallParentFunction))
  (if (not _ispanelcreated)
    (Default|ShowOpenBuildingPanel (Variables|Default|GetHUD) self (Variables|Default|GetParamsAndValues))
    (return false)))

(fn GetPostExitDialogues
  (|CallParentFunction)
  (return (Variables|Default|GetPlayerUsedHospitalDialogue)))

(fn UpdateParamsandValuesbyDifficulty
  (bind _penalty_modifier_out (|CallParentFunction))
  (bind _keys (Utilities|Map|Keys (Variables|Default|GetParamsAndValues)))
  (for _array_element _keys
    (switch Utilities|FlowControl|Switch|SwitchonE_GameParams _array_element
      (:NewEnumerator0
        _)
      (:NewEnumerator1
        _))
    (bind _floatout (CallFunction|Roundto2DecimalPlaces (* (.Value (Utilities|Map|Find (Variables|Default|GetParamsAndValues) _array_element)) _penalty_modifier_out)))
    (Utilities|Map|Add (Variables|Default|GetParamsAndValues) _array_element _floatout))
  (return _penalty_modifier_out))