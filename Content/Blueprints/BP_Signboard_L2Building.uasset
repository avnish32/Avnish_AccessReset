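; BP_Signboard_L2Building is a building signboard for restaurant-style L2 buildings, handling entry, exit and their HUD panel.
; On entry, it checks opening hours or state via IsBuildingOpen, then either snapshots player stats and puts the controller in transition, or raises a closed alert.
; On exit, it compares one stat against that snapshot to choose satisfied or unsatisfied dialogue, which DialogueHandler steps through to the HUD.
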(event Custom|OnRestaurantEntered
  (params (ParamsMap :type Map%20of%20Strings%20to%20Reals))
  (bind _returnvalue (CallFunction|IsBuildingOpen))
  (if _returnvalue
    (Variables|Default|SetStatsBeforeEntering (Variables|/Game/Blueprints/BP_GameStats.BP_GameStats_C|GetStats (Variables|Default|GetGameStats)))
    (Variables|/Game/TopDown/Blueprints/BP_TopDownController.BP_TopDownController_C|SetIsInTransition (Variables|Default|GetTop%20Down%20Controller) true)
    (Default|OnL2BuildingEntered (Variables|Default|GetHUD) self)
    (else
      (Default|RaiseAlert (Variables|Default|GetHUD) (Variables|Default|GetBuildingClosedAlertMsg)))))

(event Custom|OnRestaurantExited
  (bind _dialoguehandler (Variables|Default|GetDialogueHandler))
  (Variables|/Game/TopDown/Blueprints/BP_TopDownController.BP_TopDownController_C|SetIsInTransition (Variables|Default|GetTop%20Down%20Controller) false)
  (Default|OnRestaurantExited (Variables|Default|GetHUD))
  (bind _postexitdialogues (CallFunction|GetPostExitDialogues))
  (Variables|Default|SetCurrentDialogues _postexitdialogues)
  (Variables|Default|SetcurrentDialogueIndex -1)
  (EventDispatchers|UnbindallEventsfromOnNextDialogueDispatcher _dialoguehandler)
  (EventDispatchers|BindEventtoOnNextDialogueDispatcher _dialoguehandler (delegate Custom|AdvanceDialogue))
  (CallFunction|AdvanceDialogue))

(event Custom|AdvanceDialogue
  (bind _result (Math|Integer|IncrementInt (Variables|Default|GetcurrentDialogueIndex))
    (:%20%20
      (Default|SendDialoguetoHUD (Variables|Default|GetDialogueHandler) (Utilities|Array|Get(acopy) (Variables|Default|GetCurrentDialogues) _result))
      (if (== (Variables|Default|GetcurrentDialogueIndex) (- (Utilities|Array|Length (Variables|Default|GetCurrentDialogues)) 1))
        (Default|ResetonNextDialogueBehaviour (Variables|Default|GetDialogueHandler))))))

(event EventBeginPlay
  (|CallParentFunction)
  (EventDispatchers|BindEventtoOnBuildingEntered (delegate Custom|OnRestaurantEntered)))

(event Collision|EventActorBeginOverlap
  (params (OtherActor :type Actor%20Object%20Reference)))

(event EventTick
  (params (DeltaSeconds :type Float%20%28single-precision%29)))

(fn ConstructionScript
  (|CallParentFunction))

(fn CreateBuildingPanel
  (bind _ispanelcreated (|CallParentFunction))
  (if (not _ispanelcreated)
    (Default|ShowRestaurantPanel (Variables|Default|GetHUD) self)))

(fn HideBuildingPanel
  (Default|HideCurrentBuildingPanel (Variables|Default|GetHUD)))

(fn GetPostExitDialogues
  (if (< (.Value (Utilities|Map|Find (Variables|Default|GetStatsBeforeEntering) "NewEnumerator2")) (.Value (Utilities|Map|Find (Variables|/Game/Blueprints/BP_GameStats.BP_GameStats_C|GetStats (Variables|Default|GetGameStats)) "NewEnumerator2")))
    (return (Variables|Default|GetPlayerSatisfied_Dialogues))
    (else
      (return (Variables|Default|GetPlayerNotSatisfied_Dialogues)))))