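; Minimap controller actor that drives the HUD minimap and adds icons for signboards in the world.
; Each tick it rotates the player pointer to the character's yaw and maps the character's world position into the MPC_Minimap Offset parameter.
; When a signboard begins play, it shows the HUD panel and adds a centre-anchored icon widget sized from border and map scale, retrying next tick until player and panel are valid.
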(event Custom|OnSignboardBeginPlay
  (params (Signboard :type BP%20Signboard%20Object%20Reference))
  (bind _returnvalue (Game|GetPlayerCharacter 0))
  (bind _asbp_hud (Utilities|Casting|CastToBP_HUD (HUD|GetHUD (Game|GetPlayerController 0))))
  (bind _minimappanelout (Default|ShowMinimapPanel _asbp_hud (Variables|Default|GetMinimapBG)))
  (bind _output_get (Variables|Default|SetMinimapPanel _minimappanelout))
  (Variables|Default|SetMinimapBorderSize (Class|CanvasPanelSlot|GetSize (Class|WidgetLayoutLibrary|SlotasCanvasSlot (Variables|/Game/Blueprints/UI/BP_MinimapPanel.BP_MinimapPanel_C|GetMinimapBorder _output_get))))
  (Utilities|IsValid _returnvalue :!label _label
    (:Is%20Valid
      (bind _asbp_top_down_character (Utilities|Casting|CastToBP_TopDownCharacter _returnvalue))
      (Variables|Default|SetPlayerCharacter _asbp_top_down_character)
      (Development|PrintString (Utilities|GetDisplayName Signboard))
      (bind _returnvalue_2 (Rendering|Material|GetScalarParameterValue "/Game/Materials/MPC_Minimap.MPC_Minimap" "Scale" :!class /Script/Engine.KismetMaterialLibrary))
      (Development|PrintString (Utilities|String|ToString(Vector2d) (Math|Vector2D|MakeVector2D (* (/ 1.0 _returnvalue_2) (.X (Math|Vector2D|BreakVector2D (Variables|Default|GetMinimapBorderSize)))) (* (/ 1.0 _returnvalue_2) (.Y (Math|Vector2D|BreakVector2D (Variables|Default|GetMinimapBorderSize)))))))
      (bind _returnvalue_3 (UserInterface|CreateWidget "/Game/Blueprints/UI/BP_SignboardMinimapIcon.BP_SignboardMinimapIcon_C" 0 Signboard (Variables|Default|GetWorldMapBounds) (Math|Vector4|MakeVector4 0.0 (* (/ 1.0 _returnvalue_2) (.X (Math|Vector2D|BreakVector2D (Variables|Default|GetMinimapBorderSize)))) 0.0 (* (/ 1.0 _returnvalue_2) (.Y (Math|Vector2D|BreakVector2D (Variables|Default|GetMinimapBorderSize))))) (Variables|Default|GetPlayerCharacter) (/ (.X (Math|Vector2D|BreakVector2D (Variables|Default|GetMinimapBorderSize))) 2.0)))
      (bind _minimappanel (Variables|Default|GetMinimapPanel :!label _label_2)
        (:then
          (bind _returnvalue_4 (Widget|Panel|AddChild (Variables|/Game/Blueprints/UI/BP_MinimapPanel.BP_MinimapPanel_C|GetMinimapParentPanel _minimappanel) _returnvalue_3))
          (bind _ascanvas_panel_slot (Utilities|Casting|CastToCanvasPanelSlot _returnvalue_4))
          (Class|CanvasPanelSlot|SetAnchors _ascanvas_panel_slot (Utilities|Struct|MakeAnchors "(X=0.500000,Y=0.500000)" "(X=0.500000,Y=0.500000)"))
          (Class|CanvasPanelSlot|SetAlignment _ascanvas_panel_slot "(X=0.500000,Y=0.500000)")
          (Variables|/Script/UMG.CanvasPanelSlot|SetbAutoSize _ascanvas_panel_slot true))
        (:else
          (Utilities|FlowControl|DelayUntilNextTick)
          (goto _label_2))))
    (:Is%20Not%20Valid
      (Utilities|FlowControl|DelayUntilNextTick)
      (goto _label))))

(event EventBeginPlay
  (Utilities|FlowControl|Sequence))

(event Collision|EventActorBeginOverlap
  (params (OtherActor :type Actor%20Object%20Reference)))

(event EventTick
  (params (DeltaSeconds :type Float%20%28single-precision%29))
  (CallFunction|UpdatePlayerPtrRotation)
  (CallFunction|UpdateMinimapOffset))

(fn ConstructionScript)

(fn UpdatePlayerPtrRotation
  (bind _minimappanel (Variables|Default|GetMinimapPanel)
    (:then
      (Variables|/Script/UMG.Widget|SetRenderTransform (Variables|/Game/Blueprints/UI/BP_MinimapPanel.BP_MinimapPanel_C|GetPlayerPtr _minimappanel) (Utilities|Struct|MakeWidgetTransform (.Translation (Utilities|Struct|BreakWidgetTransform (Variables|/Script/UMG.Widget|GetRenderTransform (Variables|/Game/Blueprints/UI/BP_MinimapPanel.BP_MinimapPanel_C|GetPlayerPtr _minimappanel)))) (.Scale (Utilities|Struct|BreakWidgetTransform (Variables|/Script/UMG.Widget|GetRenderTransform (Variables|/Game/Blueprints/UI/BP_MinimapPanel.BP_MinimapPanel_C|GetPlayerPtr _minimappanel)))) (.Shear (Utilities|Struct|BreakWidgetTransform (Variables|/Script/UMG.Widget|GetRenderTransform (Variables|/Game/Blueprints/UI/BP_MinimapPanel.BP_MinimapPanel_C|GetPlayerPtr _minimappanel)))) (.Yaw (Math|Rotator|BreakRotator (Transformation|GetActorRotation (Variables|Default|GetPlayerCharacter)))))))
    (:else)))

(fn UpdateMinimapOffset
  (bind _playercharacter (Variables|Default|GetPlayerCharacter))
  (bind _worldmapbounds (Variables|Default|GetWorldMapBounds))
  (bind _minimapclampbounds (Variables|Default|GetMinimapClampBounds))
  (bind (_x _y _z _w) (Math|Vector4|BreakVector4 _worldmapbounds))
  (bind (_x_2 _y_2 _z_2 _w_2) (Math|Vector4|BreakVector4 _minimapclampbounds))
  (bind _returnvalue (Transformation|GetActorLocation _playercharacter))
  (bind (_x_3 _y_3) (Math|Vector|BreakVector _returnvalue))
  (Rendering|Material|SetVectorParameterValue "/Game/Materials/MPC_Minimap.MPC_Minimap" "Offset" (Utilities|Struct|MakeLinearColor (Math|Float|MapRangeClamped _y_3 _z _w _x_2 _y_2) (Math|Float|MapRangeClamped _x_3 _x _y _z_2 _w_2) 0.0 0.0) :!class /Script/Engine.KismetMaterialLibrary))