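; Restaurant signboard building that shows a restaurant panel on the HUD and handles the player entering and leaving the restaurant.
; On entry it flags the top-down controller as in transition and passes the name and menu to the HUD.
; On exit it clears that flag, then rebinds the dialogue handler to step through the player-satisfied lines, resetting that binding at the last one.
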(event Custom|OnRestaurantEntered
  (Variables|/Game/TopDown/Blueprints/BP_TopDownController.BP_TopDownController_C|SetIsInTransition (Variables|Default|GetTop%20Down%20Controller) true)
  (Default|OnRestaurantEntered (Variables|Default|GetHUD) (Variables|Default|GetbuildingName) (Variables|Default|GetMenu) self))

(event Custom|OnRestaurantExited
  (bind _dialoguehandler (Variables|Default|GetDialogueHandler))
  (Variables|/Game/TopDown/Blueprints/BP_TopDownController.BP_TopDownController_C|SetIsInTransition (Variables|Default|GetTop%20Down%20Controller) false)
  (Default|OnRestaurantExited (Variables|Default|GetHUD))
  (Variables|Default|SetCurrentDialogues (Variables|Default|GetPlayerSatisfied_Dialogues))
  (Variables|Default|SetcurrentDialogueIndex -1)
  (EventDispatchers|UnbindallEventsfromOnNextDialogueDispatcher _dialoguehandler)
  (EventDispatchers|BindEventtoOnNextDialogueDispatcher _dialoguehandler (delegate Custom|AdvanceDialogue))
  (CallFunction|AdvanceDialogue))

(event Custom|AdvanceDialogue
  (bind _result (Math|Integer|IncrementInt (Variables|Default|GetcurrentDialogueIndex))
    (:%20%20
      (Default|SendDialoguetoHUD (Variables|Default|GetDialogueHandler) (Utilities|Array|Get(acopy) (Variables|Default|GetCurrentDialogues) _result))
      (if (== (Variables|Default|GetcurrentDialogueIndex) (- (Utilities|Array|Length (Variables|Default|GetCurrentDialogues)) 1))
        (Default|ResetonNextDialogueBehaviour (Variables|Default|GetDialogueHandler))))))

(event EventBeginPlay
  (|CallParentFunction)
  (EventDispatchers|BindEventtoOnBuildingEntered (delegate Custom|OnRestaurantEntered)))

(event Collision|EventActorBeginOverlap
  (params (OtherActor :type Actor%20Object%20Reference)))

(event EventTick
  (params (DeltaSeconds :type Float%20%28single-precision%29)))

(fn ConstructionScript
  (|CallParentFunction))

(fn CreateBuildingPanel
  (Default|ShowRestaurantPanel (Variables|Default|GetHUD) (Variables|Default|GetbuildingName) (Variables|Default|GetRestaurantDesc) self))

(fn HideBuildingPanel
  (Default|HideRestaurantPanel (Variables|Default|GetHUD)))