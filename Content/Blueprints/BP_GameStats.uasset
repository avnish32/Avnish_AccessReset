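; BP_GameStats is an actor that holds the game's stats in an enum-keyed map, including money and time of day.
; Requested changes apply only if money stays non-negative; otherwise the HUD raises an insufficient-money alert.
; Updates add deltas, clamp percent-based stats to 0–100 and wrap time past 1440.
; A one-second looping timer advances the clock, pausing during controller transitions; the sunlight update is left unconnected.
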(event EventBeginPlay
  (bind _returnvalue (Game|GetPlayerController 0))
  (Utilities|FlowControl|Sequence
    (:then_0
      (bind _asbp_hud (Utilities|Casting|CastToBP_HUD (HUD|GetHUD _returnvalue)))
      (Variables|Default|SetHUD _asbp_hud))
    (:then_1
      (bind _asbp_top_down_controller (Utilities|Casting|CastToBP_TopDownController _returnvalue))
      (Variables|Default|SetTop%20Down%20Controller _asbp_top_down_controller))
    (:then_2
      (Utilities|Time|SetTimerbyFunctionName 0 "Update Time" 1.0 true))))

(event Collision|EventActorBeginOverlap
  (params (OtherActor :type Actor%20Object%20Reference)))

(event EventTick
  (params (DeltaSeconds :type Float%20%28single-precision%29)))

(fn ConstructionScript)

(fn ValidateandUpdateStats
  (params (ParamsAndValuesToUpdate :type Map%20of%20E_GameParams%20Enums%20to%20Reals :default "NewEnumerator0"))
  (bind (_isvalid _validationmsg) (CallFunction|ValidateStatsBeforeUpdating ParamsAndValuesToUpdate))
  (if _isvalid
    (CallFunction|UpdateStats ParamsAndValuesToUpdate)
    (return true "")
    (else
      (return _isvalid _validationmsg))))

(fn UpdateTime
  (bind _stats (Variables|Default|GetStats))
  (bind _timeprogressionrate (Variables|Default|GetTimeProgressionRate))
  (bind _stats_2 (Variables|Default|GetStats))
  (bind _value (Utilities|Map|Find _stats "NewEnumerator1"))
  (bind _returnvalue (+ _value _timeprogressionrate))
  (if (not (Variables|/Game/TopDown/Blueprints/BP_TopDownController.BP_TopDownController_C|GetIsInTransition (Variables|Default|GetTop%20Down%20Controller)))
    (if (>= _returnvalue 1.44e+03)
      (Utilities|Map|Add _stats_2 "NewEnumerator1" 0.0)
      (else
        (Utilities|Map|Add _stats_2 "NewEnumerator1" _returnvalue)))))

(fn ValidateStatsBeforeUpdating
  (params (ParamsAndValuesToUpdate :type Map%20of%20E_GameParams%20Enums%20to%20Reals :default "NewEnumerator0"))
  (bind _insuficientmoneyerrormsg (Variables|Default|GetInsuficientMoneyErrorMsg))
  (if (Utilities|Map|Contains ParamsAndValuesToUpdate "NewEnumerator0")
    (if (< (+ (.Value (Utilities|Map|Find (Variables|Default|GetStats) "NewEnumerator0")) (.Value (Utilities|Map|Find ParamsAndValuesToUpdate "NewEnumerator0"))) 0.0)
      (Development|PrintString "invalid params")
      (Default|RaiseAlert (Variables|Default|GetHUD) _insuficientmoneyerrormsg)
      (return false _insuficientmoneyerrormsg)
      (else
        _)))
  (Development|PrintString "valid params")
  (return true ""))

(fn UpdateStats
  (params (ParamsAndValuesToUpdate :type Map%20of%20E_GameParams%20Enums%20to%20Reals :default "NewEnumerator0"))
  (bind _stats (Variables|Default|GetStats))
  (bind _keys (Utilities|Map|Keys ParamsAndValuesToUpdate))
  (for _array_element _keys
    (if (Utilities|Array|ContainsItem (Variables|Default|GetpercentBasedStats) _array_element)
      (Utilities|Map|Add _stats _array_element (Math|Float|Clamp(Float) (+ (.Value (Utilities|Map|Find (Variables|Default|GetStats) _array_element)) (.Value (Utilities|Map|Find ParamsAndValuesToUpdate _array_element))) 0.0 1e+02))
      (else
        (Utilities|Map|Add _stats _array_element (+ (.Value (Utilities|Map|Find (Variables|Default|GetStats) _array_element)) (.Value (Utilities|Map|Find ParamsAndValuesToUpdate _array_element)))))))
  (|UpdateTimeAtEOD))