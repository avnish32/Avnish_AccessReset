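; Workplace signboard building that lets the player apply for its job or, once hired, work a shift there.
; Its panel shows either the other-workplace view or, for held jobs, work hours with salary and energy effects built from JobInfo.
; Applying checks a skill stat before adding the job to GameStats.
; Entering checks opening and shift end, advances time to shift end, and scales pay down and energy cost up in proportion to lateness.
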(event Custom|AfterCurrentWorkplacePanelShown
  (EventDispatchers|UnbindallEventsfromOnBuildingEntered)
  (EventDispatchers|BindEventtoOnBuildingEntered (delegate Custom|OnPlayerEntering)))

(event Custom|OnPlayerEntering
  (params (ParamsMap :type Map%20of%20Strings%20to%20Reals))
  (bind _returnvalue (CallFunction|IsBuildingOpen))
  (if _returnvalue
    (bind _returnvalue_2 (CallFunction|IsPlayeronTime))
    (if _returnvalue_2
      (CallFunction|UpdateTimeParambyShiftEndTime)
      (CallFunction|UpdateParamsifPlayerLate)
      (CallFunction|TransitionandUpdateParams)
      (else
        (Default|RaiseAlert (Variables|Default|GetHUD) (Variables|Default|GetShiftEndedMsg))))
    (else
      (Default|RaiseAlert (Variables|Default|GetHUD) (Variables|Default|GetBuildingClosedAlertMsg)))))

(event EventBeginPlay
  (|CallParentFunction)
  (Variables|Default|SetBuildingDescForOtherWorkplace (.Description (Utilities|Struct|BreakS_BuildingInfo (Variables|Default|GetBuildingInfo)))))

(event Collision|EventActorBeginOverlap
  (params (OtherActor :type Actor%20Object%20Reference)))

(event EventTick
  (params (DeltaSeconds :type Float%20%28single-precision%29)))

(fn ConstructionScript
  (|CallParentFunction))

(fn CreateBuildingPanel
  (bind _ispanelcreated (|CallParentFunction))
  (if _ispanelcreated
    (return false)
    (else
      (bind _returnvalue (CallFunction|DoesPlayerWorkHere))
      (if _returnvalue
        (bind _returnvalue_2 (CallFunction|GetBuildingDescforCurrentWorkplace))
        (Variables|Default|SetBuildingInfo (Utilities|Struct|MakeS_BuildingInfo (.Name (Utilities|Struct|BreakS_BuildingInfo (Variables|Default|GetBuildingInfo))) _returnvalue_2 (.Timings (Utilities|Struct|BreakS_BuildingInfo (Variables|Default|GetBuildingInfo))) (.Type (Utilities|Struct|BreakS_BuildingInfo (Variables|Default|GetBuildingInfo)))))
        (CallFunction|BuildParamsMapfromJobInfo)
        (Default|ShowOpenBuildingPanel (Variables|Default|GetHUD) self (Variables|Default|GetParamsAndValues))
        (CallFunction|AfterCurrentWorkplacePanelShown)
        (else
          (Variables|Default|SetBuildingInfo (Utilities|Struct|MakeS_BuildingInfo (.Name (Utilities|Struct|BreakS_BuildingInfo (Variables|Default|GetBuildingInfo))) (Variables|Default|GetBuildingDescForOtherWorkplace) (.Timings (Utilities|Struct|BreakS_BuildingInfo (Variables|Default|GetBuildingInfo))) (.Type (Utilities|Struct|BreakS_BuildingInfo (Variables|Default|GetBuildingInfo)))))
          (Default|ShowOtherWorkplacePanel (Variables|Default|GetHUD) self))))))

(fn DoesPlayerWorkHere
  (for _array_element (Variables|/Game/Blueprints/BP_GameStats.BP_GameStats_C|GetCurrentJobs (Variables|Default|GetGameStats))
    (return (Utilities|Enum|Equal(Enum) (.JobEnum (Utilities|Struct|BreakS_Job _array_element)) (.JobEnum (Utilities|Struct|BreakS_Job (Variables|Default|GetJobInfo)))))))

(fn ApplyforWork
  (bind _hud (Variables|Default|GetHUD))
  (bind _returnvalue (CallFunction|IsPlayerQualified))
  (if _returnvalue
    (Default|RaiseAlert _hud (Variables|Default|GetCongratsMsg))
    (Utilities|Array|Add (Variables|/Game/Blueprints/BP_GameStats.BP_GameStats_C|GetCurrentJobs (Variables|Default|GetGameStats)) (Variables|Default|GetJobInfo))
    (Default|HideCurrentBuildingPanel (Variables|Default|GetHUD))
    (CallFunction|CreateBuildingPanel)
    (else
      (Default|RaiseAlert _hud (Variables|Default|GetNotSkilledEnoughMsg)))))

(fn IsPlayerQualified
  (return (>= (.Value (Utilities|Map|Find (Variables|/Game/Blueprints/BP_GameStats.BP_GameStats_C|GetStats (Variables|Default|GetGameStats)) "NewEnumerator3")) (.SkillReqd (Utilities|Struct|BreakS_Job (Variables|Default|GetJobInfo))))))

(fn BuildParamsMapfromJobInfo
  (bind _jobinfo (Variables|Default|GetJobInfo))
  (bind (_jobenum _skillreqd _dailysalary _timings _dailyenergyreqd) (Utilities|Struct|BreakS_Job _jobinfo))
  (Variables|Default|SetParamsAndValues (Utilities|Map|MakeMap (Utilities|Enum|LiteralenumE_GameParams "NewEnumerator0") _dailysalary "NewEnumerator2" (* _dailyenergyreqd -1.0))))

(fn ConvertJobTimingstoString
  (bind _jobinfo (Variables|Default|GetJobInfo))
  (bind _timings (Utilities|Struct|BreakS_Job _jobinfo))
  (bind _output (Utilities|Array|Get(acopy) _timings 1))
  (bind _output_2 (Utilities|Array|Get(acopy) _timings))
  (bind (_x _y) (Math|Vector2D|BreakVector2D _output_2))
  (bind (_x_2 _y_2) (Math|Vector2D|BreakVector2D _output))
  (return (Utilities|String|ToString(Text) (Utilities|Text|FormatText "{Start.h}:{Start.m} - {End.h}:{End.m}" (Utilities|Text|ToText(Float) _x "HalfToEven" false true 2 324 0 0) (Utilities|Text|ToText(Float) _y "HalfToEven" false true 2 324 0 0) (Utilities|Text|ToText(Float) _x_2 "HalfToEven" false true 2 324 0 0) (Utilities|Text|ToText(Float) _y_2 "HalfToEven" false true 2 324 0 0)))))

(fn GetBuildingDescforCurrentWorkplace
  (bind _returnvalue (CallFunction|ConvertJobTimingstoString))
  (return (Utilities|String|ToString(Text) (Utilities|Text|FormatText "{Building desc} {Suffix} {Work hours}." (Variables|Default|GetBuildingDescForOtherWorkplace) (Variables|Default|GetBuildingDescSuffixForCurrentWorkplace) _returnvalue))))

(fn UpdateTimeParambyShiftEndTime
  (bind _jobinfo (Variables|Default|GetJobInfo))
  (bind _timings (Utilities|Struct|BreakS_Job _jobinfo))
  (bind _output (Utilities|Array|Get(acopy) _timings 1))
  (bind (_x _y) (Math|Vector2D|BreakVector2D _output))
  (Utilities|Map|Add (Variables|Default|GetParamsAndValues) "NewEnumerator1" (- (+ (* _x 6e+01) _y) (.Value (Utilities|Map|Find (Variables|/Game/Blueprints/BP_GameStats.BP_GameStats_C|GetStats (Variables|Default|GetGameStats)) "NewEnumerator1")))))

(fn UpdateParamsifPlayerLate
  (bind _jobinfo (Variables|Default|GetJobInfo))
  (bind _timings (Utilities|Struct|BreakS_Job _jobinfo))
  (bind _output (Utilities|Array|Get(acopy) _timings))
  (bind _output_2 (Utilities|Array|Get(acopy) _timings 1))
  (bind (_x _y) (Math|Vector2D|BreakVector2D _output))
  (bind (_x_2 _y_2) (Math|Vector2D|BreakVector2D _output_2))
  (bind _returnvalue (* _x 6e+01))
  (bind _returnvalue_2 (+ _returnvalue _y))
  (bind _output_get (LocalVariables|SetLateDurationInMins (- (.Value (Utilities|Map|Find (Variables|/Game/Blueprints/BP_GameStats.BP_GameStats_C|GetStats (Variables|Default|GetGameStats)) "NewEnumerator1")) _returnvalue_2)))
  (if (< _output_get 0.0)
    (return)
    (else
      (bind _output_get_2 (LocalVariables|SetShiftDurationInMins (Math|Float|Absolute(Float) (- _returnvalue_2 (+ (* _x_2 6e+01) _y_2)))))
      (LocalVariables|SetPenalty (/ _output_get _output_get_2))
      (Utilities|FlowControl|Sequence
        (:then_0
          (Utilities|Map|Add (Variables|Default|GetParamsAndValues) "NewEnumerator0" (* (.Value (Utilities|Map|Find (Variables|Default|GetParamsAndValues) "NewEnumerator0")) (- 1.0 (LocalVariables|GetPenalty)))))
        (:then_1
          (Utilities|Map|Add (Variables|Default|GetParamsAndValues) "NewEnumerator2" (* (.Value (Utilities|Map|Find (Variables|Default|GetParamsAndValues) "NewEnumerator2")) (+ 1.0 (LocalVariables|GetPenalty)))))))))

(fn IsPlayeronTime
  (bind _jobinfo (Variables|Default|GetJobInfo))
  (bind _timings (Utilities|Struct|BreakS_Job _jobinfo))
  (bind _output (Utilities|Array|Get(acopy) _timings 1))
  (bind (_x _y) (Math|Vector2D|BreakVector2D _output))
  (return (<= (.Value (Utilities|Map|Find (Variables|/Game/Blueprints/BP_GameStats.BP_GameStats_C|GetStats (Variables|Default|GetGameStats)) "NewEnumerator1")) (+ (* _x 6e+01) _y))))