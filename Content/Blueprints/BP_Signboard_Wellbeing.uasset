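; BP_Signboard_Wellbeing is a signboard for a wellbeing building that shows a generic HUD panel and changes game stats when the building is entered.
; On entry, GameStats validates ParamsAndValues, printing the validation message on failure.
; On success, a timed sequence hides the panel, shows a transition message, flags the TopDownController as in transition, applies the stats, then ends the transition.
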(event Custom|OnWellbeingEntered
  (bind (_isvalid _validationmsg) (Default|ValidateStatsBeforeUpdating (Variables|Default|GetGameStats) (Variables|Default|GetParamsAndValues)))
  (if _isvalid
    (Default|HideBuildingPanel (Variables|Default|GetHUD))
    (Default|OnGenericBuildingEntered (Variables|Default|GetHUD) (Variables|Default|GetTransitionMsg))
    (Utilities|FlowControl|Delay 1.0)
    (Variables|/Game/TopDown/Blueprints/BP_TopDownController.BP_TopDownController_C|SetIsInTransition (Variables|Default|GetTop%20Down%20Controller) true)
    (Utilities|FlowControl|Delay 1.0)
    (CallFunction|UpdateGameStats)
    (Development|PrintString "Stats updated")
    (Utilities|FlowControl|Delay 2.0)
    (Variables|/Game/TopDown/Blueprints/BP_TopDownController.BP_TopDownController_C|SetIsInTransition (Variables|Default|GetTop%20Down%20Controller) false)
    (Default|OnTransitionCompleted (Variables|Default|GetHUD))
    (else
      (Development|PrintString _validationmsg))))

(event EventBeginPlay
  (|CallParentFunction)
  (EventDispatchers|BindEventtoOnBuildingEntered (delegate Custom|OnWellbeingEntered)))

(event Collision|EventActorBeginOverlap
  (params (OtherActor :type Actor%20Object%20Reference)))

(event EventTick
  (params (DeltaSeconds :type Float%20%28single-precision%29)))

(fn ConstructionScript
  (|CallParentFunction))

(fn CreateBuildingPanel
  (Default|ShowGenericBuildingPanel (Variables|Default|GetHUD) (Variables|Default|GetbuildingName) (Variables|Default|GetParamsAndValues) self))

(fn UpdateGameStats
  (Default|UpdateStats (Variables|Default|GetGameStats) (Variables|Default|GetParamsAndValues)))

(fn HideBuildingPanel
  (Default|HideBuildingPanel (Variables|Default|GetHUD)))