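; BP_Signboard is a proximity-triggered signboard that calls building-panel functions when the top-down character enters or leaves its sphere.
; BeginPlay caches the HUD, game stats actor and player controller, then unbinds all events from OnBuildingEntered.
; Sphere overlaps call CreateBuildingPanel and HideBuildingPanel, but both functions, like UpdateGameStats, are empty here.
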(event OnComponentBeginOverlap(Sphere)
  (params (OverlappedComponent :type Primitive%20Component%20Object%20Reference) (OtherActor :type Actor%20Object%20Reference) (OtherComp :type Primitive%20Component%20Object%20Reference) (OtherBodyIndex :type Integer) (bFromSweep :type Boolean) (SweepResult :type Hit%20Result%20Structure%20%28by%20ref%29))
  (Utilities|Casting|CastToBP_TopDownCharacter OtherActor)
  (CallFunction|CreateBuildingPanel))

(event OnComponentEndOverlap(Sphere)
  (params (OverlappedComponent :type Primitive%20Component%20Object%20Reference) (OtherActor :type Actor%20Object%20Reference) (OtherComp :type Primitive%20Component%20Object%20Reference) (OtherBodyIndex :type Integer))
  (Utilities|Casting|CastToBP_TopDownCharacter OtherActor)
  (CallFunction|HideBuildingPanel))

(event EventBeginPlay
  (Utilities|FlowControl|Sequence
    (:then_0
      (bind _asbp_hud (Utilities|Casting|CastToBP_HUD (HUD|GetHUD (Game|GetPlayerController 0))))
      (Variables|Default|SetHUD _asbp_hud))
    (:then_1
      (bind _returnvalue (Actor|GetActorOfClass "/Game/Blueprints/BP_GameStats.BP_GameStats_C"))
      (Variables|Default|SetGameStats _returnvalue))
    (:then_2
      (bind _asbp_top_down_controller (Utilities|Casting|CastToBP_TopDownController (Game|GetPlayerController 0)))
      (Variables|Default|SetTop%20Down%20Controller _asbp_top_down_controller))
    (:then_3
      (EventDispatchers|UnbindallEventsfromOnBuildingEntered))))

(fn ConstructionScript)

(fn UpdateGameStats)

(fn CreateBuildingPanel)

(fn HideBuildingPanel)