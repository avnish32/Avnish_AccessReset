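; Main menu game mode that ensures a save game exists when the menu starts.
; On BeginPlay it casts to BP_GameInstance and checks for a save using that instance's slot name and user index.
; If none exists, it looks up a fixed default difficulty row in DT_DifficultyModes by enum name and passes it to the game instance's SaveGame function.
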(event EventBeginPlay
  (bind _asbp_game_instance (Utilities|Casting|CastToBP_GameInstance (Game|GetGameInstance)))
  (bind _returnvalue (SaveGame|DoesSaveGameExist (Variables|/Game/Blueprints/BP_GameInstance.BP_GameInstance_C|GetSaveGameSlotName _asbp_game_instance) (Variables|/Game/Blueprints/BP_GameInstance.BP_GameInstance_C|GetSaveGameUserIndex _asbp_game_instance)))
  (if (not _returnvalue)
    (bind _returnvalue_2 (Utilities|GetDataTableRow "/Game/Data/DT_DifficultyModes.DT_DifficultyModes" (Utilities|String|StringToName (Utilities|String|EnumtoString (Utilities|Enum|LiteralenumE_DiffcultyModes "NewEnumerator1"))))
      (:then
        (Default|SaveGame _asbp_game_instance _returnvalue_2)))))

(event EventTick
  (params (DeltaSeconds :type Float%20%28single-precision%29)))

(fn ConstructionScript)